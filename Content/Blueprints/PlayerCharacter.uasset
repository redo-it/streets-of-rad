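; Player character for a side-scrolling Paper2D game, with movement, HUD, overlap-based melee and radiation-fuelled mutations.
; Holding Mutate turns the three attack inputs into two-tier upgrade purchases, using slots earned from radiation.
; Tick selects the flipbook, revokes the newest mutations when radiation drops, and derives damage, speed, ranged and special stats from mutation flags.
; Ranged attack is a stub; a debug toggle prints flags and adjusts radiation.
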(event `InputAction|Crouch`
  (params (Key :type "Key Structure"))
  ;[1 1 1] Basic Movement
  (:`Pressed`
    (`self.Crouch`))
  (:`Released`
    (`self.UnCrouch`)))

(event `InputAction|Jump`
  (params (Key :type "Key Structure"))
  ;[1 1 1] Basic Movement
  (:`Pressed`
    (`self.Jump`))
  (:`Released`
    (`self.StopJumping`)))

(event `InputAxis|LRAxis`
  (params (AxisValue :type "Float (single-precision)"))
  ;[1 1 1] Basic Movement
  (`self.AddMovementInput` (1.0 0.0 0.0) (* AxisValue (`self.PlayerSpeed`))))

(event `self.ReceiveBeginPlay`
  (bind _returnvalue (`|CreateWidget` "/Game/Ui/hud.hud_C"))
  (`UserWidget.AddToViewport` _returnvalue 0))

(event `InputAction|BasicAttack`
  (params (Key :type "Key Structure"))
  (bind _mutationstatus (`self.MutationStatus`))
  (bind _mutationsactive (`self.MutationsActive`))
  ;[1 1 1] Combat
  (:`Pressed`
    (if (`self.MutationMode`)
      ;[1 1 1] Mutation
      (if (> (stale `self.ReceiveTick` _output_get) 0)
        (if (`|GetArrayItem` _mutationstatus)
          (`KismetArrayLibrary.Array_Set` _mutationstatus 1 true)
          (`KismetArrayLibrary.Array_Add` _mutationsactive 1)
          (else
            (`KismetArrayLibrary.Array_Set` _mutationstatus 0 true)
            (`KismetArrayLibrary.Array_Add` _mutationsactive))))
      (elif (not (`self.isAttacking`))
        (set `self.isAttacking` true)
        (for _array_element (`self.GetOverlappingActors` "/Game/Blueprints/MasterEnemy.MasterEnemy_C")
          (bind _asmaster_enemy (cast `/Game/Blueprints/MasterEnemy` _array_element))
          (set `/Game/Blueprints/MasterEnemy.Health` (- (`/Game/Blueprints/MasterEnemy.Health` _asmaster_enemy) (`self.PlayerDamage`)) _asmaster_enemy)
          (`KismetSystemLibrary.Delay` 0.5)
          (set `self.isAttacking` false))))))

(event `InputAction|RangedAttack`
  (params (Key :type "Key Structure"))
  (bind _mutationstatus (`self.MutationStatus`))
  (bind _mutationsactive (`self.MutationsActive`))
  ;[1 1 1] Combat
  (:`Pressed`
    (if (`self.MutationMode`)
      ;[1 1 1] Mutation
      (if (> (stale `self.ReceiveTick` _output_get) 0)
        (if (`|GetArrayItem` _mutationstatus 2)
          (`KismetArrayLibrary.Array_Set` _mutationstatus 3 true)
          (`KismetArrayLibrary.Array_Add` _mutationsactive 3)
          (else
            (`KismetArrayLibrary.Array_Set` _mutationstatus 2 true)
            (`KismetArrayLibrary.Array_Add` _mutationsactive 2))))
      (elif (`self.RangedAttackPossible`)
        _))))

(event `InputAction|SpecialAttack`
  (params (Key :type "Key Structure"))
  (bind _mutationstatus (`self.MutationStatus`))
  (bind _mutationsactive (`self.MutationsActive`))
  ;[1 1 1] Combat
  (:`Pressed`
    (if (`self.MutationMode`)
      ;[1 1 1] Mutation
      (if (> (stale `self.ReceiveTick` _output_get) 0)
        (if (`|GetArrayItem` _mutationstatus 4)
          (`KismetArrayLibrary.Array_Set` _mutationstatus 5 true)
          (`KismetArrayLibrary.Array_Add` _mutationsactive 5)
          (else
            (`KismetArrayLibrary.Array_Set` _mutationstatus 4 true)
            (`KismetArrayLibrary.Array_Add` _mutationsactive 4)))))))

(event `InputAction|Mutate`
  (params (Key :type "Key Structure"))
  ;[1 1 1] Mutation
  (:`Pressed`
    (set `self.MutationMode` true))
  (:`Released`
    (set `self.MutationMode` false)))

(event `InputAction|DebugToggle`
  (params (Key :type "Key Structure"))
  (bind _debugmode (`self.DebugMode`))
  ;[1 1 1] Debug
  (:`Pressed`
    (if _debugmode
      (set `self.DebugMode` false)
      (else
        (set `self.DebugMode` true)
        (for _array_element (`self.MutationStatus`) :!label _label
          (`KismetSystemLibrary.PrintString` (`KismetStringLibrary.Conv_BoolToString` _array_element))
          (`KismetSystemLibrary.Delay` 2.0)
          (set `self.RadiationAmount` (+ (`self.RadiationAmount`) 2))
          (if _debugmode
            (goto _label)))))))

(event `InputAction|SpecialAttack`
  (params (Key :type "Key Structure"))
  ;[1 1 1] Debug
  (:`Pressed`
    (if (`self.DebugMode`)
      (set `self.RadiationAmount` 0))))

(event `self.ReceiveTick`
  (params (DeltaSeconds :type "Float (single-precision)"))
  (bind _mutationsactive (`self.MutationsActive`))
  (bind _mutationstatus (`self.MutationStatus`))
  (bind _returnvalue (`KismetArrayLibrary.Array_LastIndex` _mutationsactive))
  (bind _returnvalue_2 (- (/ (`self.RadiationAmount`) 25) (`KismetArrayLibrary.Array_Length` (`self.MutationsActive`))))
  ;[1 1 1] Mutation
  (`self.AnimationStateMachine`)
  (bind _output_get (set `self.MutationsAvailable` _returnvalue_2))
  (while (< _output_get 0)
    (`KismetArrayLibrary.Array_Set` _mutationstatus (`|GetArrayItem` _mutationsactive _returnvalue))
    (`KismetArrayLibrary.Array_Remove` _mutationsactive _returnvalue)
    (set `self.MutationsAvailable` _returnvalue_2))
  (if (`|GetArrayItem` _mutationstatus)
    (if (`|GetArrayItem` _mutationstatus 1)
      (set `self.PlayerDamage` 3)
      (else
        (set `self.PlayerDamage` 2)))
    (else
      (set `self.PlayerDamage` 1)))
  (if (`|GetArrayItem` _mutationstatus 2)
    (if (`|GetArrayItem` _mutationstatus 3)
      (set `self.PlayerSpeed` 2.25)
      (else
        (set `self.PlayerSpeed` 1.5)))
    (else
      (set `self.PlayerSpeed` 1.0)))
  (if (`|GetArrayItem` _mutationstatus 4)
    (if (`|GetArrayItem` _mutationstatus 5)
      (set `self.SpecialChargeSpeed` 2)
      (else
        (set `self.RangedAttackPossible` true)))
    (else
      (set `self.RangedAttackPossible` false)
      (set `self.SpecialChargeSpeed` 1))))

(fn `AnimationStateMachine`
  (bind _playerflipbook (`self.PlayerFlipbook`))
  (if (`self.isAttacking`)
    (`PaperFlipbookComponent.SetFlipbook` _playerflipbook "/Game/Sprites/Attack.Attack")
    (elif (`NavMovementComponent.IsFalling` (`self.CharacterMovement`))
      (`PaperFlipbookComponent.SetFlipbook` _playerflipbook "/Game/Sprites/Jumping.Jumping")
      (elif (> (`KismetMathLibrary.VSize` (`self.GetVelocity`)) 0.0)
        (`PaperFlipbookComponent.SetFlipbook` _playerflipbook "/Game/Sprites/Walking.Walking")
        (else
          (`PaperFlipbookComponent.SetFlipbook` _playerflipbook "/Game/Sprites/Idle.Idle")
          (return))))))

(fn `UserConstructionScript`)