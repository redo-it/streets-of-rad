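; MasterEnemy is a flipbook-animated enemy, by its name a base class, that moves toward the player and can be killed.
; A DealDamage event subtracts Health, and Tick destroys the actor at zero or below, otherwise adding slow movement input toward player 0.
; AnimationStateMachine picks attack, jump, walk or idle flipbooks from IsAttacking, falling state and velocity.
; Nothing in this graph calls that function or sets IsAttacking.
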(event `DealDamage`
  (params (Amount :type Integer))
  (set `self.Health` (- (`self.Health`) Amount)))

(event `self.ReceiveTick`
  (params (DeltaSeconds :type "Float (single-precision)"))
  (if (<= (`self.Health`) 0)
    (`self.K2_DestroyActor`)
    (else
      (`self.AddMovementInput` (`KismetMathLibrary.Normal` (- (`self.K2_GetActorLocation` (`GameplayStatics.GetPlayerCharacter` 0)) (`self.K2_GetActorLocation`))) 0.1))))

(fn `AnimationStateMachine`
  (bind _playerflipbook (`self.PlayerFlipbook`))
  (if (`self.isAttacking`)
    (`PaperFlipbookComponent.SetFlipbook` _playerflipbook "/Game/Sprites/PlayerCharacter/Attack.Attack")
    (elif (`NavMovementComponent.IsFalling` (`self.CharacterMovement`))
      (`PaperFlipbookComponent.SetFlipbook` _playerflipbook "/Game/Sprites/PlayerCharacter/Jumping.Jumping")
      (elif (> (`KismetMathLibrary.VSize` (`self.GetVelocity`)) 0.0)
        (`PaperFlipbookComponent.SetFlipbook` _playerflipbook "/Game/Sprites/PlayerCharacter/Walking.Walking")
        (else
          (`PaperFlipbookComponent.SetFlipbook` _playerflipbook "/Game/Sprites/PlayerCharacter/Idle.Idle")
          (return))))))

(fn `UserConstructionScript`)